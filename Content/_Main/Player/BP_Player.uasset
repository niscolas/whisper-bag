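; Player Blueprint that owns the inventory, dialogue and input-help UI and links it to its inventory and interactor components.
; On BeginPlay it creates the widgets and registers inventory and dialogue MVVM viewmodels in the global collection.
; Component events push items and dialogue lines into the viewmodels, while inventory viewmodel removals call back into the component.
; Dialogue blends the camera to the trigger actor and back, and an input action toggles inventory and input mode.
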(event `self.ReceiveBeginPlay`
  ;[1 1 1] BeginPlay
  (`self.SetupInventoryViewmodel`)
  (`self.SetupDialogueViewmodel`)
  (`self.SetupCommonInputHelpHUD`)
  (`self.SetupInventoryUI`)
  (`self.SetupDialoguePanel`)
  (add `/Game/_Main/UI/WBP_DialoguePanel.DialogueEnded` (`self.DialoguePanel`) (`|CreateDelegate` :!event `OnDialogueEnded`)))

(event `EnhancedInput|/Game/_Main/Input/IA_OpenInventory`
  (params (ActionValue :type Boolean) (ElapsedSeconds :type "Float (double-precision)") (TriggeredSeconds :type "Float (double-precision)") (InputAction :type "InputAction Object Reference" :default "/Game/_Main/Input/IA_OpenInventory.IA_OpenInventory"))
  ;[1 1 1] IA_OpenInventory
  (:`Triggered`
    (if ActionValue
      (switch `ESlateVisibility` (`Widget.GetVisibility` (`self.FullInventoryUi`))
        (:`Visible`
          (`self.DisableInventoryUI`))
        (:`Collapsed`
          (`self.EnableInventoryUI`))))))

(event `self.InventoryComponent.InventoryUpdated`
  ;[1 1 1] OnInventoryUpdated
  (bind _returnvalue (`InventoryComponent.GetItemsAsArray` (`self.InventoryComponent`)))
  (set `/Game/_Main/Player/VM_Inventory.Items` _returnvalue (`self.VM_Inventory`)))

(event `self.InteractorComponent.NewDialogueTriggered`
  (params (DialogueLines :type "Array of Text") (DialogueTriggerActor :type "DialogueTrigger Object Reference"))
  ;[1 1 1] OnNewDialogueTriggered
  (set `/Game/_Main/Player/VM_Dialogue.DialogueLines` DialogueLines (`self.VM_Dialogue`))
  (`PlayerController.SetViewTargetWithBlend` (`GameplayStatics.GetPlayerController` 0) DialogueTriggerActor 1.0 "VTBlend_EaseInOut" 2.0 false))

(event `OnDialogueEnded`
  ;[1 1 1] OnDialogueEnded
  (set `/Game/_Main/Player/VM_Dialogue.DialogueLines` (`|MakeArray`) (`self.VM_Dialogue`))
  (`PlayerController.SetViewTargetWithBlend` (`GameplayStatics.GetPlayerController` 0) self 1.0 "VTBlend_EaseInOut" 2.0 false))

(event `OnInventoryViewmodelRemovedItemChanged`
  (params (Object :type "Object Object Reference") (Field :type "FieldNotificationId Structure"))
  (`InventoryComponent.RemoveItem` (`self.InventoryComponent`) (`/Game/_Main/Player/VM_Inventory.RemovedItem` (`self.VM_Inventory`))))

(fn `DisableInventoryUI`
  (`/Game/_Main/Libraries/BlueprintFunctionLibraries/BPFL_Input.ActivateGameInputMode` (`GameplayStatics.GetPlayerControllerFromID` 0))
  (`Widget.SetVisibility` (`self.FullInventoryUi`) "Collapsed"))

(fn `EnableInventoryUI`
  (`/Game/_Main/Libraries/BlueprintFunctionLibraries/BPFL_Input.ActivateGameInputMode` (`GameplayStatics.GetPlayerControllerFromID` 0) false true)
  (`Widget.SetVisibility` (`self.FullInventoryUi`) "Visible"))

(fn `SetupCommonInputHelpHUD`
  (bind _returnvalue (`|CreateWidget` "/Game/_Main/UI/WBP_CommonInputHelpHud.WBP_CommonInputHelpHud_C"))
  (bind _output_get (set `self.CommonInputHelpHUD` _returnvalue))
  (`UserWidget.AddToViewport` _output_get 0))

(fn `SetupDialoguePanel`
  (bind _returnvalue (`|CreateWidget` "/Game/_Main/UI/WBP_DialoguePanel.WBP_DialoguePanel_C"))
  (bind _output_get (set `self.DialoguePanel` _returnvalue))
  (`UserWidget.AddToViewport` _output_get 0)
  (`Widget.SetVisibility` (`self.DialoguePanel`) "Collapsed"))

(fn `SetupDialogueViewmodel`
  (bind _returnvalue (`|GenericCreateObject` "/Game/_Main/Player/VM_Dialogue.VM_Dialogue_C"))
  (bind _output_get (set `self.VM_Dialogue` _returnvalue))
  (`MVVMViewModelCollectionObject.AddViewModelInstance` (`MVVMGameSubsystem.GetViewModelCollection` (subsystem `MVVMGameSubsystem`)) (make `MVVMViewModelContext` "/Game/_Main/Player/VM_Dialogue.VM_Dialogue_C" "VM_Dialogue") _output_get))

(fn `SetupInventoryUI`
  (bind _returnvalue (`|CreateWidget` "/Game/_Main/UI/WBP_FullInventoryUi.WBP_FullInventoryUi_C"))
  (bind _output_get (set `self.FullInventoryUi` _returnvalue))
  (`UserWidget.AddToViewport` _output_get 0)
  (`Widget.SetVisibility` _output_get "Collapsed"))

(fn `SetupInventoryViewmodel`
  (bind _returnvalue (`|GenericCreateObject` "/Game/_Main/Player/VM_Inventory.VM_Inventory_C"))
  (bind _output_get (set `self.VM_Inventory` _returnvalue))
  (`MVVMViewModelCollectionObject.AddViewModelInstance` (`MVVMGameSubsystem.GetViewModelCollection` (subsystem `MVVMGameSubsystem`)) (make `MVVMViewModelContext` "/Game/_Main/Player/VM_Inventory.VM_Inventory_C" "VM_Inventory") _output_get)
  (`MVVMViewModelBase.K2_AddFieldValueChangedDelegate` (`self.VM_Inventory`) (struct :`FieldName` "RemovedItem") (`|CreateDelegate` :!event `OnInventoryViewmodelRemovedItemChanged`)))

(fn `UserConstructionScript`)